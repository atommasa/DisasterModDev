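; A map marker action that toggles tracking of the selected marker for the player.
; On execute it asks the MapTrackingSubsystem whether the context point's ID is tracked, then clears or tracks it and completes as succeeded.
; The display name switches between "Track" and "Stop Tracking" from the same check, and the action is always available.
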(event EventExecuteAction
  (params (Context :type Game%20Zone%20Marker%20Action%20Context%20Structure%20%28by%20ref%29))
  (bind _pointid (Utilities|Struct|BreakGameZonePointData (.point Context)))
  (bind _returnvalue (Subsystems|GetMapTrackingSubsystem (.playercontroller Context)))
  (if (Class|MapTrackingSubsystem|IsMarkerTracked _returnvalue _pointid)
    (Class|MapTrackingSubsystem|ClearTrackedMarker _returnvalue)
    (else
      (Class|MapTrackingSubsystem|TrackMarker _returnvalue _pointid)))
  (Class|GameZoneMarkerAction|CompleteAction (Utilities|Struct|MakeGameZoneMarkerActionResult "Succeeded" "")))

(fn GetAvailability
  (params (Context :type Game%20Zone%20Marker%20Action%20Context%20Structure%20%28by%20ref%29))
  (return (Utilities|Struct|MakeGameZoneMarkerActionAvailabilityResult "Available" "")))

(fn GetDisplayName
  (params (Context :type Game%20Zone%20Marker%20Action%20Context%20Structure%20%28by%20ref%29) (DefaultDisplayName :type Text%20%28by%20ref%29))
  (if (Class|MapTrackingSubsystem|IsMarkerTracked (Subsystems|GetMapTrackingSubsystem (.playercontroller Context)) (Utilities|Struct|BreakGameZonePointData (.point Context)))
    (return "Stop Tracking")
    (else
      (return "Track"))))