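; Marker action that fast-travels the player to the game zone of a map marker point.
; Executing it calls EnterGameZone on the GameZoneSubsystem with the point's zone and entry ID, using the saved world transform when the point ID is invalid, then reports success immediately.
; The action is available only for activated markers and hidden for deactivated or hidden ones.
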(event EventExecuteAction
  (params (Context :type Game%20Zone%20Marker%20Action%20Context%20Structure%20%28by%20ref%29))
  (bind (_pointid _zoneid _markertypeid _markertags _markerstate _displaymode _savepolicy _displayname _description _referenceassetid _worldtransform) (Utilities|Struct|BreakGameZonePointData (.point Context)))
  (Class|GameZoneSubsystem|EnterGameZone (Subsystems|GetGameZoneSubsystem (.playercontroller Context)) (Utilities|Struct|MakeGameZoneContext _zoneid (not (Guid|IsValidGuid _pointid)) (Utilities|Struct|MakeGameZoneEntryId _pointid) _worldtransform))
  (Class|GameZoneMarkerAction|CompleteAction (Utilities|Struct|MakeGameZoneMarkerActionResult "Succeeded" "")))

(fn GetAvailability
  (params (Context :type Game%20Zone%20Marker%20Action%20Context%20Structure%20%28by%20ref%29))
  (switch Utilities|FlowControl|Switch|SwitchonEGameZonePointState (Utilities|Struct|BreakGameZonePointData (.point Context))
    (:Activated
      (return (Utilities|Struct|MakeGameZoneMarkerActionAvailabilityResult "Available" "")))
    (:Deactivated
      _)
    (:Hide
      _))
  (return (Utilities|Struct|MakeGameZoneMarkerActionAvailabilityResult "Hidden" "")))