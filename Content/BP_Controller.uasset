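; BP_Controller is a controller with test key bindings for saving, loading and party spawning.
; E and Q call the save game subsystem to synchronously save or load the "Test" slot.
; F has the character subsystem spawn NewParty members at the controlled pawn's location with zero rotation.
; An unconnected leftover chain would apply a gameplay effect to the first BP_Character's ability system component and print a message.
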(event EventBeginPlay)

(event Input|KeyboardEvents|E
  (params (Key :type Key%20Structure :default "None"))
  (:Pressed
    (Class|SaveGameSubsystem|SaveGame (Subsystems|GetSaveGameSubsystem) "Test" false)))

(event Input|KeyboardEvents|F
  (params (Key :type Key%20Structure :default "None"))
  (:Pressed
    (Class|CharacterSubsystem|SpawnNewPartyMembers (Subsystems|GetCharacterSubsystem) (Variables|Default|GetNew%20Party) (Transformation|GetActorLocation (Pawn|GetControlledPawn)) "0, 0, 0")))

(event Input|KeyboardEvents|Q
  (params (Key :type Key%20Structure :default "None"))
  (:Pressed
    (Class|SaveGameSubsystem|LoadGame (Subsystems|GetSaveGameSubsystem) "Test" false)))

(fn ConstructionScript)