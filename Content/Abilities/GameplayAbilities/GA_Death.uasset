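; GA_Death is the gameplay ability that handles a character's death.
; On activation it has the avatar's CombatComponent initialize a post-death hit reaction, plays phase 0 and ends when that completes, is interrupted or is cancelled.
; Without a CombatComponent it cancels itself.
; When the ability ends, it disables capsule collision and AI control on the BaseCharacter, then tells the CombatComponent to finish death.
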(event Ability|EventActivateAbility
  (bind _returnvalue (Ability|GetAvatarActorfromActorInfo))
  (bind _returnvalue_2 (Actor|GetComponentbyClass _returnvalue "/Script/RPGCore.CombatComponent"))
  (Utilities|IsValid _returnvalue_2
    (:Is%20Valid
      (Class|CombatComponent|InitializePostDeathHitReaction _returnvalue_2)
      (|PlayPhaseandWaitProxy "None" 0 "(ComboWindowOpenEventTag=(TagName=\"\"),ComboWindowCloseEventTag=(TagName=\"\"),ComboTransitionEventTag=(TagName=\"\"),AllowedInputTags=(GameplayTags=),bBlockOtherInputsDuringComboWindow=True,InputListenerPriority=100)"
        (:OnCompleted
          _)
        (:OnInterrupted
          _)
        (:OnCancelled
          _))
      (Ability|EndAbility))
    (:Is%20Not%20Valid
      (Ability|CancelAbility))))

(event Ability|EventOnEndAbility
  (params (bWasCancelled :type Boolean))
  (bind _asbase_character (Utilities|Casting|CastToBaseCharacter (Ability|GetAvatarActorfromActorInfo)))
  (Collision|SetCollisionEnabled (Variables|/Script/Engine.Character|GetCapsuleComponent _asbase_character) "NoCollision")
  (Class|BaseCharacter|SetAIControl _asbase_character false)
  (Class|CombatComponent|FinishDeath (Variables|/Script/RPGCore.BaseCharacter|GetCombatComponent _asbase_character)))